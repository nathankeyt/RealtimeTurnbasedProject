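; Music manager component that plays a queue of looping MetaSound songs with crossfades and adjustable intensity.
; It adds two audio components to its owner and alternates them on each song change or loop, letting reverb tails overlap.
; Tick compares wall-clock playtime to clip length minus tail to advance the queue or repeat its last song, and drives volume fades.
; It also blends an Intensity parameter into both sources.
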(event EventBeginPlay
  (bind _output_get (Variables|Default|SetActor (Components|GetOwner)))
  (bind _returnvalue (Game|AddComponentbyClass _output_get "/Script/Engine.AudioComponent" false))
  (Audio|Components|Audio|Stop _returnvalue)
  (Variables|Default|SetAudioSource1 _returnvalue)
  (bind _returnvalue_2 (Game|AddComponentbyClass _output_get "/Script/Engine.AudioComponent" false))
  (Audio|Components|Audio|Stop _returnvalue_2)
  (Variables|Default|SetAudioSource2 _returnvalue_2))

(event EventTick
  (params (DeltaSeconds :type Float%20%28single-precision%29))
  (bind _returnvalue (|CurrentPlaytime_2))
  (bind _returnvalue_2 (|TotalPlayTime-RT_2))
  (bind _lastsound (Variables|Default|GetLastSound))
  (bind _volume (Variables|Default|GetVolume))
  (bind _fadingsource (Variables|Default|GetFadingSource))
  (bind _playingsource (Variables|Default|GetPlayingSource))
  (bind _pendingsounds (Variables|Default|GetPendingSounds))
  (bind _output (Utilities|Array|Get(acopy) _pendingsounds))
  (bind _returnvalue_3 (!= _output _lastsound))
  (Utilities|FlowControl|Sequence
    (:then_0
      (if (!= (Utilities|Array|Length (Variables|Default|GetPendingSounds)) 0)
        (if _returnvalue_3
          (CallFunction|NextSong)
          (else
            (Utilities|FlowControl|Sequence
              (:then_0
                (if (and (< (Variables|Default|GetLast%20PlayTime) _returnvalue_2) (> _returnvalue _returnvalue_2))
                  (CallFunction|NextSong)))
              (:then_1
                (Variables|Default|SetLast%20PlayTime _returnvalue)))))
        (else
          (CallFunction|NextSong))))
    (:then_1
      (Utilities|IsValid (Variables|Default|GetPlayingSource)
        (:Is%20Valid
          (Utilities|IsValid (Variables|Default|GetFadingSource)
            (:Is%20Valid
              (if (== (Variables|Default|GetCurTransitionTime) -1.0)
                (Audio|Components|Audio|SetVolumeMultiplier _fadingsource _volume :!class /Script/Engine.AudioComponent :!label _label)
                (Audio|Components|Audio|SetVolumeMultiplier _playingsource _volume :!class /Script/Engine.AudioComponent)
                (elif (> (stale _output_get) 0.0)
                  (bind _output_get (Variables|Default|SetCurTransitionTime (- (stale _output_get) DeltaSeconds)))
                  (Audio|Components|Audio|SetVolumeMultiplier _fadingsource (* (/ _output_get (Variables|Default|GetCurTransitionTimeMax)) _volume) :!class /Script/Engine.AudioComponent)
                  (Audio|Components|Audio|SetVolumeMultiplier _playingsource (* (- 1.0 (/ _output_get (Variables|Default|GetCurTransitionTimeMax))) _volume) :!class /Script/Engine.AudioComponent)
                  (elif _returnvalue_3
                    (goto _label)))))))))
    (:then_2
      (bind _output_get_2 (Variables|Default|SetIntensityCurTime (+ (stale _output_get_2) DeltaSeconds)))
      (Audio|Parameter|SetFloatParameter (Variables|Default|GetAudioSource1) "Intensity" (Math|Float|Lerp (Variables|Default|GetIntensityStart) (Variables|Default|GetIntensityTarg) (Math|Float|Clamp(Float) (/ _output_get_2 (Variables|Default|GetIntensityBlendTime)))) :!class /Script/AudioExtensions.AudioParameterControllerInterface)
      (Audio|Parameter|SetFloatParameter (Variables|Default|GetAudioSource2) "Intensity" (Math|Float|Lerp (Variables|Default|GetIntensityStart) (Variables|Default|GetIntensityTarg) (Math|Float|Clamp(Float) (/ _output_get_2 (Variables|Default|GetIntensityBlendTime)))) :!class /Script/AudioExtensions.AudioParameterControllerInterface)
      (if (>= (Math|Float|Clamp(Float) (/ _output_get_2 (Variables|Default|GetIntensityBlendTime))) 1.0)
        (Variables|Default|SetIntensityStart (Variables|Default|GetIntensityTarg))))))

(event Custom|Next%20Song
  (bind _pendingsounds (Variables|Default|GetPendingSounds))
  (bind _pendingsounds_loopnum (Variables|Default|GetPendingSounds_LoopNum))
  (bind _pendingsounds_fadetime (Variables|Default|GetPendingSounds_FadeTime))
  (bind _pendingsounds_2 (Variables|Default|GetPendingSounds))
  (bind _returnvalue (Utilities|Array|Length _pendingsounds))
  (bind _output (Utilities|Array|Get(acopy) _pendingsounds_fadetime))
  (if (!= _returnvalue 0)
    (if (!= (Variables|Default|GetLastSound) 0)
      (if (== _returnvalue 1)
        _
        (else
          (Utilities|Array|RemoveIndex _pendingsounds_2)
          (Utilities|Array|RemoveIndex (Variables|Default|GetPendingSounds_MainLengths))
          (Utilities|Array|RemoveIndex (Variables|Default|GetPendingSounds_TailLengths))
          (Utilities|Array|RemoveIndex _pendingsounds_loopnum)
          (Utilities|Array|RemoveIndex _pendingsounds_fadetime)))
      (CallFunction|Swap&Play (Utilities|Array|Get(acopy) _pendingsounds_2) :!label _label)
      (Audio|Parameter|SetFloatParameter (Variables|Default|GetPlayingSource) "LoopNum" (/ (Math|Conversions|ToFloat(Integer) (Utilities|Array|Get(acopy) _pendingsounds_loopnum)) 2.0) :!class /Script/Engine.AudioComponent)
      (bind _output_get (Variables|Default|SetCurTransitionTime (Math|Float|SelectFloat 0.025 _output (== _output 0.0))))
      (Variables|Default|SetCurTransitionTimeMax _output_get)
      (else
        (Utilities|FlowControl|Sequence
          (:then_0
            (goto _label))
          (:then_1
            (bind _output_get_2 (Variables|Default|SetCurTransitionTime -1.0))
            (Variables|Default|SetCurTransitionTimeMax _output_get_2)))))
    (else
      (CallFunction|Swap&Play)
      (Audio|Components|Audio|SetSound (Variables|Default|GetPlayingSource) 0))))

(event Custom|Swap&Play
  (params (Meta%20Sound :type Meta%20Sound%20Source%20Object%20Reference))
  (bind _audiosource1 (Variables|Default|GetAudioSource1))
  (bind _audiosource2 (Variables|Default|GetAudioSource2))
  (Variables|Default|SetPlayStartTime (Math|DateTime|Now))
  (bind _output_get (Variables|Default|SetCurrentSource (== (Variables|Default|GetCurrentSource) false)))
  (if _output_get
    (Utilities|IsValid Meta%20Sound
      (:Is%20Valid
        (Audio|Components|Audio|SetSound _audiosource1 Meta%20Sound)
        (Variables|Default|SetLastSound Meta%20Sound))
      (:Is%20Not%20Valid
        _))
    (Audio|Components|Audio|Play _audiosource1 0.0)
    (Variables|Default|SetPlayingSource _audiosource1)
    (Variables|Default|SetFadingSource _audiosource2)
    (else
      (Utilities|IsValid Meta%20Sound
        (:Is%20Valid
          (Audio|Components|Audio|SetSound _audiosource2 Meta%20Sound)
          (Variables|Default|SetLastSound Meta%20Sound))
        (:Is%20Not%20Valid
          _))
      (Audio|Components|Audio|Play _audiosource2 0.0)
      (Variables|Default|SetPlayingSource _audiosource2)
      (Variables|Default|SetFadingSource _audiosource1))))

(fn PlayLoopingSong
  (params (Song :type Meta%20Sound%20Source%20Object%20Reference) (Clip%20Length :type Float%20%28double-precision%29) (Reverb%20Tail%20Length :type Float%20%28double-precision%29) (Clip%20Alts%20Selection :type Integer) (Play%20Now%20/%20Clear%20Queue :type Boolean) (Play%20Now%20Fade%20Time :type Float%20%28double-precision%29))
  (if Play%20Now%20/%20Clear%20Queue
    (Variables|Default|SetPendingSounds (Utilities|Array|MakeArray Song))
    (Variables|Default|SetPendingSounds_MainLengths (Utilities|Array|MakeArray Clip%20Length))
    (Variables|Default|SetPendingSounds_TailLengths (Utilities|Array|MakeArray Reverb%20Tail%20Length))
    (Variables|Default|SetPendingSounds_LoopNum (Utilities|Array|MakeArray Clip%20Alts%20Selection))
    (Variables|Default|SetPendingSounds_FadeTime (Utilities|Array|MakeArray Play%20Now%20Fade%20Time))
    (else
      (Utilities|Array|Add (Variables|Default|GetPendingSounds) Song)
      (Utilities|Array|Add (Variables|Default|GetPendingSounds_MainLengths) Clip%20Length)
      (Utilities|Array|Add (Variables|Default|GetPendingSounds_TailLengths) Reverb%20Tail%20Length)
      (Utilities|Array|Add (Variables|Default|GetPendingSounds_LoopNum) Clip%20Alts%20Selection)
      (Utilities|Array|Add (Variables|Default|GetPendingSounds_FadeTime) (Math|Float|SelectFloat (Math|Float|SelectFloat 0.025 Play%20Now%20Fade%20Time (== Play%20Now%20Fade%20Time 0.0)) -1.0 Play%20Now%20/%20Clear%20Queue)))))

(fn SkipSongs
  (params (Amount :type Integer) (TransitionTime :type Float%20%28double-precision%29))
  (bind _returnvalue (- Amount 1))
  (if (>= _returnvalue (Utilities|Array|Length (Variables|Default|GetPendingSounds)))
    (Utilities|Array|Clear (Variables|Default|GetPendingSounds))
    (Utilities|Array|Clear (Variables|Default|GetPendingSounds_MainLengths))
    (Utilities|Array|Clear (Variables|Default|GetPendingSounds_TailLengths))
    (Utilities|Array|Clear (Variables|Default|GetPendingSounds_LoopNum))
    (Utilities|Array|Clear (Variables|Default|GetPendingSounds_FadeTime))
    (else
      (for _index (range 0 _returnvalue)
        (Utilities|Array|RemoveIndex (Variables|Default|GetPendingSounds))
        (Utilities|Array|RemoveIndex (Variables|Default|GetPendingSounds_MainLengths))
        (Utilities|Array|RemoveIndex (Variables|Default|GetPendingSounds_TailLengths))
        (Utilities|Array|RemoveIndex (Variables|Default|GetPendingSounds_LoopNum))
        (Utilities|Array|RemoveIndex (Variables|Default|GetPendingSounds_FadeTime)))
      (Utilities|Array|SetArrayElem (Variables|Default|GetPendingSounds_FadeTime) 0 (Math|Float|SelectFloat 0.001 TransitionTime (== TransitionTime 0.0)))
      (CallFunction|NextSong))))

(fn SetIntensity0-1
  (params (Intensity :type Float%20%28double-precision%29) (Blend%20Time :type Float%20%28double-precision%29))
  (Variables|Default|SetIntensityTarg (* Intensity 2.0))
  (Variables|Default|SetIntensityBlendTime (Math|Float|SelectFloat 0.0001 Blend%20Time (== Blend%20Time 0.0)))
  (Variables|Default|SetIntensityCurTime 0.0))