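; Player character that creates an ability display HUD and, on the R key, switches the turn through the game mode while toggling a cinematic ability sequence.
; Toggling on shows an animated ability widget, plays a montage, and uses a timeline to swing and zoom the camera while fading in a post-process outline mask.
; When the timeline finishes, the view blends to the locked-on enemy; toggling off resets control rotation and camera boom.
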(event EventBeginPlay
  (bind _returnvalue (UserInterface|CreateWidget "/Game/UI/Widgets/AbilityDisplayWidget_BP.AbilityDisplayWidget_BP_C"))
  (bind _output_get (Variables|Default|SetAbilityDisplay _returnvalue))
  (UserInterface|Viewport|AddtoViewport _output_get 0)
  (Class|AbilityDisplayWidget|SetAbilityDisplay (Variables|Default|GetAbilityDisplay) (Variables|Default|GetAbilitySystem)))

(event Input|KeyboardEvents|R
  (params (Key :type Key%20Structure :default "None"))
  (:Pressed
    (bind _asmain_game_mode_bp (Utilities|Casting|CastToMainGameMode_BP (Game|GetGameMode)))
    (Class|MainGameMode|SwitchTurn _asmain_game_mode_bp "TE_PlayerTurn")
    (if (Variables|Default|GetToggle)
      (Variables|Default|SetToggle false)
      (Variables|Default|SetbUseControllerRotationYaw false)
      (Pawn|SetControlRotation (Pawn|GetController) (Transformation|GetActorRotation))
      (Variables|/Script/Engine.SpringArmComponent|SetTargetArmLength (Variables|Default|GetCameraBoom) 3e+02)
      (Variables|/Script/Engine.SpringArmComponent|SetSocketOffset (Variables|Default|GetCameraBoom) "0, 0, 0")
      (else
        (bind _returnvalue (UserInterface|CreateWidget "/Game/UI/Widgets/AbilityAnimationWidget_BP.AbilityAnimationWidget_BP_C"))
        (bind _output_get (Variables|Default|SetAnimationUI _returnvalue))
        (UserInterface|Viewport|AddtoViewport _output_get 0)
        (UserInterface|Animation|PlayAnimation (Variables|Default|GetAnimationUI) (Variables|/Game/UI/Widgets/AbilityAnimationWidget_BP.AbilityAnimationWidget_BP_C|GetGrow (Variables|Default|GetAnimationUI)) 0.0 1 "Forward" 1.0 false)
        (UserInterface|Animation|PlayAnimation (Variables|Default|GetAnimationUI) (Variables|/Game/UI/Widgets/AbilityAnimationWidget_BP.AbilityAnimationWidget_BP_C|GetText (Variables|Default|GetAnimationUI)) 0.0 1 "Forward" 1.0 false)
        (bind _returnvalue_2 (Rendering|Material|CreateDynamicMaterialInstance "/Game/Materials/PPMaterials/PPM_PlayerOutline.PPM_PlayerOutline" "None" "None" :!class /Script/Engine.KismetMaterialLibrary))
        (bind _output_get_2 (Variables|Default|SetMask _returnvalue_2))
        (Variables|/Script/Engine.CameraComponent|SetPostProcessSettings (Variables|Default|GetFollowCamera) (Utilities|Struct|MakePostProcessSettings (Utilities|Struct|MakeWeightedBlendables (Utilities|Array|MakeArray (Utilities|Struct|MakeWeightedBlendable 1.0 _output_get_2)))))
        (Animation|PlayAnimMontage 0 1.0 "None")
        (Variables|Default|SetToggle true)
        (Variables|Default|SetbUseControllerRotationYaw false)
        (bind _alpha (Timeline|Timeline Play)
          (:Update
            (Pawn|SetControlRotation (Pawn|GetController) (Math|Rotator|Lerp(Rotator) (Transformation|GetActorRotation) (Math|Rotator|CombineRotators (Transformation|GetActorRotation) "-5.000000,170.000000,0.000000") _alpha))
            (Variables|/Script/Engine.SpringArmComponent|SetSocketOffset (Variables|Default|GetCameraBoom) (Math|Vector|Lerp(Vector) "0, 0, 0" "0.000000,0.000000,55.000000" _alpha))
            (Variables|/Script/Engine.SpringArmComponent|SetTargetArmLength (Variables|Default|GetCameraBoom) (Math|Float|Lerp 3e+02 2e+02 _alpha))
            (Rendering|Material|SetScalarParameterValue (Variables|Default|GetMask) "MaskAlpha" _alpha :!class /Script/Engine.MaterialInstanceDynamic))
          (:Finished
            (bind _asenemy_character_bp (Utilities|Casting|CastToEnemyCharacter_BP (Variables|Default|GetLockOnTarget)))
            (Game|Player|SetViewTargetwithBlend (Game|GetPlayerController 0) _asenemy_character_bp 1.0 "VTBlend_Cubic" 0.0 false)))))))

(fn ConstructionScript)